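; MasterTile is an endless-runner track tile with three lanes that spawns obstacles and extends the track.
; On BeginPlay, nested random switches check left, middle, then right lane, spawning at most one Block1 or Jump1 with a limited lifespan, favouring earlier lanes.
; When ThirdPersonCharacter overlaps the Box trigger, the tile asks ThirdPersonGameMode to spawn another tile, then destroys itself after a short delay.
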(event OnComponentBeginOverlap(Box)
  (params (OverlappedComponent :type Primitive%20Component%20Object%20Reference) (OtherActor :type Actor%20Object%20Reference) (OtherComp :type Primitive%20Component%20Object%20Reference) (OtherBodyIndex :type Integer) (bFromSweep :type Boolean) (SweepResult :type Hit%20Result%20Structure%20%28by%20ref%29))
  (Utilities|Casting|CastToThirdPersonCharacter OtherActor)
  (bind _asthird_person_game_mode (Utilities|Casting|CastToThirdPersonGameMode (Game|GetGameMode)))
  (Default|SpawnTile _asthird_person_game_mode)
  (Utilities|FlowControl|Delay 0.5)
  (Actor|DestroyActor))

(event EventBeginPlay
  (CallFunction|SpawnObsticals))

(event Collision|EventActorBeginOverlap
  (params (OtherActor :type Actor%20Object%20Reference)))

(event EventTick
  (params (DeltaSeconds :type Float%20%28single-precision%29)))

(fn ConstructionScript)

(fn SpawnObsticals
  (bind _leftlane (Variables|Default|GetLeftLane))
  (bind _middlelane (Variables|Default|GetMiddleLane))
  (bind _rightlane (Variables|Default|GetRightLane))
  (bind _returnvalue (Transformation|GetWorldTransform _rightlane))
  (bind _returnvalue_2 (Transformation|GetWorldTransform _leftlane))
  (bind _returnvalue_3 (Transformation|GetWorldTransform _middlelane))
  ;[1 1 1] LeftLane
  (switch int (Math|Random|RandomIntegerinRange 0 5)
    (:Default
      ;[1 1 1] MiddleLane
      (switch int (Math|Random|RandomIntegerinRange 0 5)
        (:Default
          ;[1 1 1] RightLane
          (switch int (Math|Random|RandomIntegerinRange 0 5)
            (:0
              (bind _returnvalue_4 (Game|SpawnActorfromClass "/Game/RunnerFiles/Blueprint/Block1.Block1_C" _returnvalue "Undefined" 0 0))
              (Actor|SetLifeSpan _returnvalue_4 8.0))
            (:1
              (bind _returnvalue_5 (Game|SpawnActorfromClass "/Game/RunnerFiles/Blueprint/Jump1.Jump1_C" _returnvalue "Undefined" 0 0))
              (Actor|SetLifeSpan _returnvalue_5 8.0))))
        (:0
          (bind _returnvalue_6 (Game|SpawnActorfromClass "/Game/RunnerFiles/Blueprint/Block1.Block1_C" _returnvalue_3 "Undefined" 0 0))
          (Actor|SetLifeSpan _returnvalue_6 8.0))
        (:1
          (bind _returnvalue_7 (Game|SpawnActorfromClass "/Game/RunnerFiles/Blueprint/Jump1.Jump1_C" _returnvalue_3 "Undefined" 0 0))
          (Actor|SetLifeSpan _returnvalue_7 8.0))))
    (:0
      (bind _returnvalue_8 (Game|SpawnActorfromClass "/Game/RunnerFiles/Blueprint/Block1.Block1_C" _returnvalue_2 "Undefined" 0 0))
      (Actor|SetLifeSpan _returnvalue_8 8.0))
    (:1
      (bind _returnvalue_9 (Game|SpawnActorfromClass "/Game/RunnerFiles/Blueprint/Jump1.Jump1_C" _returnvalue_2 "Undefined" 0 0))
      (Actor|SetLifeSpan _returnvalue_9 8.0))))